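; Water level manager actor that syncs the water height to the first-person player's visuals and drives water movement audio.
; Each tick it writes WaterLevel into the player's intersection material and feeds normalized water depth from PlayerWaterAudio to both sounds as DistanceToCamera.
; The rising sound starts once when the level exceeds a fixed threshold and stops below it, while an OnWaterLowering event plays the lowering sound.
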(event EventBeginPlay
  (bind _outactors (Actor|GetAllActorsOfClass "/Game/FirstPerson/Blueprints/BP_FirstPersonCharacter.BP_FirstPersonCharacter_C"))
  (Variables|Default|SetPlayerRef (Utilities|Array|Get(acopy) _outactors)))

(event EventOnWaterLowering
  (Components|Activation|Activate (Variables|Default|GetWater_Lowering) true)
  (Class|FMODAudioComponent|Play (Variables|Default|GetWater_Lowering)))

(event EventTick
  (params (DeltaSeconds :type Float%20%28single-precision%29))
  (bind _playerref (Variables|Default|GetPlayerRef))
  (bind _playerwateraudio (Variables|/Game/FirstPerson/Blueprints/BP_FirstPersonCharacter.BP_FirstPersonCharacter_C|GetPlayerWaterAudio _playerref))
  (bind _returnvalue (Class|PlayerWaterAudio|GetNormalizedWaterDepth _playerwateraudio))
  (Rendering|Material|SetScalarParameterValue (Variables|/Game/FirstPerson/Blueprints/BP_FirstPersonCharacter.BP_FirstPersonCharacter_C|GetMID_Intersection (Variables|Default|GetPlayerRef)) "WaterPlaneZ" (Variables|Default|GetWaterLevel) :!class /Script/Engine.MaterialInstanceDynamic)
  (Utilities|FlowControl|Sequence
    (:then_0
      (Class|FMODAudioComponent|SetParameter (Variables|Default|GetWater_Rising) "DistanceToCamera" _returnvalue)
      (Class|FMODAudioComponent|SetParameter (Variables|Default|GetWater_Lowering) "DistanceToCamera" _returnvalue))
    (:then_1
      (Math|Float|CompareFloat (Variables|Default|GetWaterLevel) -55.0
        (:>
          (if (not (Variables|Default|GetIsPlayingRising))
            (Components|Activation|Activate (Variables|Default|GetWater_Rising) true)
            (Class|FMODAudioComponent|Play (Variables|Default|GetWater_Rising))
            (Variables|Default|SetIsPlayingRising true)))
        (:<
          (Variables|Default|SetIsPlayingRising false)
          (Class|FMODAudioComponent|Stop (Variables|Default|GetWater_Rising)))))))

(fn ConstructionScript)