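; BP_Valve is a water valve actor that, once detached, switches its indicator diodes and drives the wetness of brick materials.
; On the first Tick with ValveDetached set, it turns the red diode off and green on, copies the WaterLevelManager's level to Peak Water Level and zeroes Wetness.
; Later Ticks ramp Wetness up to 1, writing it to the Bricks_Global_Parameters material parameter collection.
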(event EventBeginPlay)

(event Collision|EventActorBeginOverlap
  (params (OtherActor :type Actor%20Object%20Reference)))

(event EventTick
  (params (DeltaSeconds :type Float%20%28single-precision%29))
  (if (Variables|Default|GetbValveDetached)
    (if (Variables|Default|GetChanged)
      (Math|Float|CompareFloat (Variables|Default|GetWetness) 1.0
        (:<
          (bind _output_get (Variables|Default|SetWetness (Math|Float|Min(Float) (+ (Variables|Default|GetWetness) (* DeltaSeconds (Variables|Default|GetWetness%20Change%20Speed))) 1.0)))
          (Rendering|Material|SetScalarParameterValue "/Game/Materials/Bricks_Global_Parameters.Bricks_Global_Parameters" "Wetness" _output_get :!class /Script/Engine.KismetMaterialLibrary)))
      (else
        (|DiodeChange)
        (Rendering|Material|SetScalarParameterValue "/Game/Materials/Bricks_Global_Parameters.Bricks_Global_Parameters" "Peak Water Level" (Variables|/Script/LodzGame.WaterLevelManager|GetWaterLevel (Variables|Default|GetWaterLevelManager)) :!class /Script/Engine.KismetMaterialLibrary)
        (bind _output_get_2 (Variables|Default|SetWetness 0.0))
        (Rendering|Material|SetScalarParameterValue "/Game/Materials/Bricks_Global_Parameters.Bricks_Global_Parameters" "Wetness" _output_get_2 :!class /Script/Engine.KismetMaterialLibrary)))))

(fn ConstructionScript)