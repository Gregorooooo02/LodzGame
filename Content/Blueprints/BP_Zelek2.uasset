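; BP_Zelek2 is an actor that acts as a slowing zone, sharply reducing the player's walk speed and jump height inside its Sphere1 component.
; On BeginPlay it caches player 0's max speed and jump velocity.
; Overlaps by actors whose root component is tagged "plajer" apply low fixed values to player 0's movement, and ending the overlap restores the cached ones.
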(event OnComponentBeginOverlap(Sphere1)
  (params (OverlappedComponent :type Primitive%20Component%20Object%20Reference) (OtherActor :type Actor%20Object%20Reference) (OtherComp :type Primitive%20Component%20Object%20Reference) (OtherBodyIndex :type Integer) (bFromSweep :type Boolean) (SweepResult :type Hit%20Result%20Structure%20%28by%20ref%29))
  (bind _returnvalue (Game|GetPlayerCharacter 0))
  (bind _charactermovement (Variables|/Script/Engine.Character|GetCharacterMovement _returnvalue))
  (if (Components|ComponentHasTag (Variables|/Script/Engine.Actor|GetRootComponent OtherActor) "plajer")
    (Variables|/Script/Engine.CharacterMovementComponent|SetJumpZVelocity _charactermovement 35.0)
    (Variables|/Script/Engine.CharacterMovementComponent|SetMaxWalkSpeed _charactermovement 75.0)))

(event OnComponentEndOverlap(Sphere1)
  (params (OverlappedComponent :type Primitive%20Component%20Object%20Reference) (OtherActor :type Actor%20Object%20Reference) (OtherComp :type Primitive%20Component%20Object%20Reference) (OtherBodyIndex :type Integer))
  (bind _returnvalue (Game|GetPlayerCharacter 0))
  (bind _charactermovement (Variables|/Script/Engine.Character|GetCharacterMovement _returnvalue))
  (if (Components|ComponentHasTag (Variables|/Script/Engine.Actor|GetRootComponent OtherActor) "plajer")
    (Variables|/Script/Engine.CharacterMovementComponent|SetJumpZVelocity _charactermovement (Variables|Default|GetMax%20Jump))
    (Variables|/Script/Engine.CharacterMovementComponent|SetMaxWalkSpeed _charactermovement (Variables|Default|GetMax%20Speed))))

(event EventBeginPlay
  (bind _returnvalue (Game|GetPlayerCharacter 0))
  (bind _charactermovement (Variables|/Script/Engine.Character|GetCharacterMovement _returnvalue))
  (Variables|Default|SetMax%20Speed (Class|MovementComponent|GetMaxSpeed _charactermovement))
  (Variables|Default|SetMax%20Jump (Variables|/Script/Engine.CharacterMovementComponent|GetJumpZVelocity _charactermovement)))

(event Collision|EventActorBeginOverlap
  (params (OtherActor :type Actor%20Object%20Reference)))

(event EventTick
  (params (DeltaSeconds :type Float%20%28single-precision%29)))

(fn ConstructionScript)