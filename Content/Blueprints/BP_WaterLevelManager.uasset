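; BP_WaterLevelManager raises a water body actor in steps over time.
; Tick accumulates elapsed time and, once it reaches RiseInterval, resets the timer and adds RisePerSecond to WaterLevel.
; It then moves WaterBody to that height, keeping X and Y and clamping only the applied Z to MaxWaterLevel, so the stored level keeps growing.
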(event EventTick
  (params (DeltaSeconds :type Float%20%28single-precision%29))
  (bind _waterbody (Variables|Default|GetWaterBody))
  (bind _returnvalue (Transformation|GetActorLocation _waterbody))
  (bind (_x _y) (Math|Vector|BreakVector _returnvalue))
  (bind _output_get (Variables|Default|SetTimeElapsed (+ DeltaSeconds (Variables|Default|GetTimeElapsed))))
  (Math|Float|CompareFloat _output_get (Variables|Default|GetRiseInterval)
    (:>
      _)
    (:==
      _))
  (Variables|Default|SetTimeElapsed 0.0)
  (bind _output_get_2 (Variables|Default|SetWaterLevel (+ (Variables|Default|GetWaterLevel) (Variables|Default|GetRisePerSecond))))
  (Transformation|SetActorLocation _waterbody (Math|Vector|MakeVector _x _y (Math|Float|Clamp(Float) _output_get_2 -1e+02 (Variables|Default|GetMaxWaterLevel))) false false))

(fn ConstructionScript)