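; Blueprint that fades an underwater post-process effect in and out based on the player's height relative to the water.
; Each tick, it compares the player pawn's Z plus HeightOffset against WaterLevelManager.WaterLevel to set a target weight of fully on or off.
; The current weight lerps toward that target, scaled by LerpSpeed and delta time, and drives the PostProcess blend weight.
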(event EventTick
  (params (DeltaSeconds :type Float%20%28single-precision%29))
  (Math|Float|CompareFloat (+ (.Z (Math|Vector|BreakVector (Transformation|GetActorLocation (Game|Player|GetPlayerPawn 0)))) (Variables|Default|GetHeightOffset)) (Variables|/Script/LodzGame.WaterLevelManager|GetWaterLevel (Variables|Default|GetWaterLevelManager))
    (:>
      (Variables|Default|SetTargetBlendWeight 0.0))
    (:<
      (Variables|Default|SetTargetBlendWeight 1.0)))
  (bind _output_get (Variables|Default|SetCurrentBlendWeight (Math|Float|Lerp (Variables|Default|GetCurrentBlendWeight) (Variables|Default|GetTargetBlendWeight) (* (Variables|Default|GetLerpSpeed) DeltaSeconds))))
  (Variables|/Script/Engine.PostProcessComponent|SetBlendWeight (Variables|Default|GetPostProcess) _output_get))

(fn ConstructionScript)