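; BP_MenuPawn is the main menu pawn, carrying a camera and a spotlight that react over time and to the mouse.
; Each tick the spotlight eases its rotation toward the point under the cursor, found by a complex visibility trace.
; The camera's relative rotation follows sine waves of game time at different frequencies per axis, giving a subtle idle sway.
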(event EventTick
  (params (DeltaSeconds :type Float%20%28single-precision%29))
  (bind _returnvalue (Utilities|Time|GetGameTimeinSeconds))
  (bind _spotlight (Variables|Default|GetSpotLight))
  (Transformation|SetWorldRotation _spotlight (Math|Interpolation|RInterpTo (Transformation|GetWorldRotation _spotlight) (Math|Rotator|FindLookatRotation (Transformation|GetWorldLocation _spotlight) (.Location (Collision|BreakHitResult (.HitResult (Game|Player|GetHitResultUnderCursorbyChannel (Game|GetPlayerController 0) "TraceTypeQuery1" true))))) DeltaSeconds 5.0) false false)
  (Transformation|SetRelativeRotation (Variables|Default|GetCamera) (Math|Rotator|MakeRotator (Math|Trig|Sin(Radians) (* _returnvalue 0.01)) (Math|Trig|Sin(Radians) (* _returnvalue 1.0)) (Math|Trig|Sin(Radians) (* _returnvalue 0.5))) false false))

(fn ConstructionScript)